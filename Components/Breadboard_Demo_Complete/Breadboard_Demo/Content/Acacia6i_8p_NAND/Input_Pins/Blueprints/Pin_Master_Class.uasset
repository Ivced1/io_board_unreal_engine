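; Master input pin actor for a NAND logic simulation, toggled on and off by the player.
; While an actor overlaps it, player input is enabled, so the 1 key drives a FlipFlop that sets the PinIn boolean.
; The pin mesh turns green for on and red for off, and the value is passed to the PinOut reference through GetValueOutput.
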(event Collision|EventActorBeginOverlap
  (params (OtherActor :type Actor%20Object%20Reference))
  ;[1 1 1] Convert this to a parent class then instantiate from the parent.
  ;;[1 1 1] Enable / Disable User Controller
  (Input|EnableInput (Game|GetPlayerController 0)))

(event Collision|EventActorEndOverlap
  (params (OtherActor :type Actor%20Object%20Reference))
  ;[1 1 1] Convert this to a parent class then instantiate from the parent.
  ;;[1 1 1] Enable / Disable User Controller
  (Input|DisableInput (Game|GetPlayerController 0)))

(event Input|KeyboardEvents|1
  (params (Key :type Key%20Structure))
  ;[1 1 1] Convert this to a parent class then instantiate from the parent.
  ;;[1 1 1] Toggle Pin on/off. Signal user with red - off, green - on.
  (:Pressed
    (Utilities|FlowControl|FlipFlop
      (:A
        (Variables|Default|SetPin_In true)
        (Rendering|Material|SetMaterial (Variables|Default|GetPin) 0 "/Game/Input_Pins/Materials/Green.Green"))
      (:B
        (Variables|Default|SetPin_In false)
        (Rendering|Material|SetMaterial (Variables|Default|GetPin) 0 "/Game/Input_Pins/Materials/Red.Red")))
    ;;[1 1 1] Send value to next blueprint - Boolean. Change this to send signal to correct pin number.
    (Default|GetValueOutput (Variables|Default|GetPin_out) (Variables|Default|GetPin_In))))

(fn ConstructionScript)