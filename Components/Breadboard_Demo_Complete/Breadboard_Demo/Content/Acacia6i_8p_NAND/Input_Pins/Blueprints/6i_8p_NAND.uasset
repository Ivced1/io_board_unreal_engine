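; Logic Blueprint for one three-input NAND gate with a single output, part of the 6i_8p_NAND asset.
; Three Get_Pin events each store their boolean input, then share one evaluation that outputs false only when all three pins are true.
; The result is pushed to the next Blueprint through GetValueOutput on PinOut, so the gate re-evaluates on each input event without using Tick.
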(event Custom|Get_Pin_3
  (params (Pin3 :type Boolean))
  ;[1 1 1] Create input events / set pins
  (bind _output_get (Variables|Default|SetPin%203 Pin3))
  ;[1 1 1] 3 Input 2 Circuit NAND Gate - Boolean
  (if (and (and (stale Custom|Get_Pin_1 _output_get) (stale Custom|Get_Pin_2 _output_get)) _output_get)
    ;[1 1 1] Send Output to next blueprint - Boolean
    (Variables|Default|SetPin_Value false)
    (else
      (Variables|Default|SetPin_Value true)))
  (Default|GetValueOutput (Variables|Default|GetPin_Out) (Variables|Default|GetPin_Value)))

(event Custom|Get_Pin_1
  (params (Pin1 :type Boolean))
  ;[1 1 1] Create input events / set pins
  (bind _output_get (Variables|Default|SetPin%201 Pin1))
  ;[1 1 1] 3 Input 2 Circuit NAND Gate - Boolean
  (if (and (and _output_get (stale Custom|Get_Pin_2 _output_get)) (stale Custom|Get_Pin_3 _output_get))
    ;[1 1 1] Send Output to next blueprint - Boolean
    (Variables|Default|SetPin_Value false)
    (else
      (Variables|Default|SetPin_Value true)))
  (Default|GetValueOutput (Variables|Default|GetPin_Out) (Variables|Default|GetPin_Value)))

(event Custom|Get_Pin_2
  (params (Pin2 :type Boolean))
  ;[1 1 1] Create input events / set pins
  (bind _output_get (Variables|Default|SetPin%202 Pin2))
  ;[1 1 1] 3 Input 2 Circuit NAND Gate - Boolean
  (if (and (and (stale Custom|Get_Pin_1 _output_get) _output_get) (stale Custom|Get_Pin_3 _output_get))
    ;[1 1 1] Send Output to next blueprint - Boolean
    (Variables|Default|SetPin_Value false)
    (else
      (Variables|Default|SetPin_Value true)))
  (Default|GetValueOutput (Variables|Default|GetPin_Out) (Variables|Default|GetPin_Value)))

(event EventBeginPlay)

(event Collision|EventActorBeginOverlap
  (params (OtherActor :type Actor%20Object%20Reference)))

(event EventTick
  (params (DeltaSeconds :type Float%20%28single-precision%29)))

(fn ConstructionScript)