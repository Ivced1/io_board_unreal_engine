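; Input pin actor for a NAND logic gate setup, letting the player toggle a boolean signal.
; While an actor overlaps it, player controller 0's input is enabled on the pin, and disabled when the overlap ends.
; Pressing the 1 key flip-flops PinIn, swaps the pin material between green (true) and red (false), and passes the value to PinOut through GetValueOutput.
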(event Collision|EventActorBeginOverlap
  (params (OtherActor :type Actor%20Object%20Reference))
  ;[1 1 1] Enable / Disable Player Controller
  (Input|EnableInput (Game|GetPlayerController 0)))

(event Collision|EventActorEndOverlap
  (params (OtherActor :type Actor%20Object%20Reference))
  ;[1 1 1] Enable / Disable Player Controller
  (Input|DisableInput (Game|GetPlayerController 0)))

(event Input|KeyboardEvents|1
  (params (Key :type Key%20Structure))
  ;[1 1 1] Pass Boolean Value to Logic Gate
  (:Pressed
    (Utilities|FlowControl|FlipFlop
      (:A
        (Variables|Default|SetPin_In true)
        (Rendering|Material|SetMaterial (Variables|Default|GetPin) 0 "/Game/Input_Pins/Materials/Green.Green"))
      (:B
        (Variables|Default|SetPin_In false)
        (Rendering|Material|SetMaterial (Variables|Default|GetPin) 0 "/Game/Input_Pins/Materials/Red.Red")))
    (Default|GetValueOutput (Variables|Default|GetPin_out) (Variables|Default|GetPin_In))))

(fn ConstructionScript)