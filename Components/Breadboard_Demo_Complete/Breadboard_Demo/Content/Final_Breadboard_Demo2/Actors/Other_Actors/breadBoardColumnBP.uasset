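; Breadboard column actor that acts as a shared electrical node, passing power between the pins overlapping it.
; Each Tick it queries overlapping actors, sends its current state to input and in/out pins, and ORs the power read from pinBP pins.
; That result, or AlwaysOn, becomes the new state, so pins receive the previously computed value.
; The column's material shows green when powered and red otherwise.
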(event EventTick
  (params (DeltaSeconds :type Float%20%28single-precision%29))
  (bind _column (Variables|Default|Getcolumn))
  (bind _column_2 (Variables|Default|Getcolumn))
  ;[0 0 0] Check for pin connections
  (bind (_outactors _returnvalue) (Collision|ComponentOverlapActors _column_2 (Transformation|GetWorldTransform _column_2) (Utilities|Array|MakeArray "ObjectTypeQuery2") 0))
  (if _returnvalue
    _
    (else
      (Variables|Default|SetisPowered (Variables|Default|GetAlwaysOn))))
  ;[0 0 0] Check each of the overlapping objects to determine if they are output pins or input by casting them. If they are outputs, add them to the list of incoming power. If they are inputs send them a power update of the column's current power status. If it is an input and output, do both.
  (for _array_element _outactors
    (bind _aspin_bpin (Utilities|Casting|CastTopinBPIn _array_element)
      (:then
        (Default|InputPower _aspin_bpin (Variables|Default|GetisPowered)))
      (:CastFailed
        (bind _aspin_bpin_out (Utilities|Casting|CastTopinBPInOut _array_element)
          (:then
            (Default|InputPower _aspin_bpin_out (Variables|Default|GetisPowered)))
          (:CastFailed
            _))))
    (bind _aspin_bp (Utilities|Casting|CastTopinBP _array_element))
    ;;[0 0.01932 1] Compare each input against each previous input. if any are true, the loopcheck sets to true
    (Variables|Default|SetLoopCheck (or (Variables|/Game/Final_Breadboard_Demo2/Actors/Other_Actors/pinBP.pinBP_C|GetisPowered _aspin_bp) (Variables|Default|GetLoopCheck))))
  ;[0 0.01781 1] Set ispowered if input is true, loop check is for each column
  (bind _output_get (Variables|Default|SetisPowered (or (Variables|Default|GetAlwaysOn) (Variables|Default|GetLoopCheck))))
  (Variables|Default|SetLoopCheck false)
  (if _output_get
    (Rendering|Material|SetMaterial _column 0 "/Game/Acacia6i_8p_NAND/Input_Pins/Materials/Green.Green")
    (else
      (Rendering|Material|SetMaterial _column 0 "/Game/Acacia6i_8p_NAND/Input_Pins/Materials/Red.Red"))))

(fn ConstructionScript)