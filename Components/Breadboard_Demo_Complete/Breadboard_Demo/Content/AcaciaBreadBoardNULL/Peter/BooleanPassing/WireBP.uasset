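; Wire Blueprint for a breadboard boolean power-passing system, linking two in/out pins as a bidirectional connection.
; The construction script registers the wire as main on both child-actor pins and gives each an ID.
; PowerUpdate switches on the pin number, stores the incoming power and outputs it through the opposite pin.
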(event EventPowerUpdate
  (params (power :type Boolean%20%28by%20ref%29) (pinNumber :type Integer%20%28by%20ref%29))
  (switch int pinNumber
    (:0
      (bind _output_get (Variables|Default|Setinput1 power))
      (bind _aspin_bp (Utilities|Casting|CastTopinBP (Variables|/Script/Engine.ChildActorComponent|GetChildActor (Variables|Default|GetpinBPInOut1))))
      (Default|OutputPower _aspin_bp _output_get))
    (:1
      (bind _output_get_2 (Variables|Default|Setinput0 power))
      (bind _aspin_bp_2 (Utilities|Casting|CastTopinBP (Variables|/Script/Engine.ChildActorComponent|GetChildActor (Variables|Default|GetpinBPInOut0))))
      (Default|OutputPower _aspin_bp_2 _output_get_2))))

(fn ConstructionScript
  (|CallParentFunction)
  (bind _aspin_bpin_out (Utilities|Casting|CastTopinBPInOut (Variables|/Script/Engine.ChildActorComponent|GetChildActor (Variables|Default|GetpinBPInOut1))))
  (Default|SetMain _aspin_bpin_out self)
  (Variables|/Game/Final_Breadboard_Demo2/Actors/Other_Actors/pinBPInOut.pinBPInOut_C|SetpinID _aspin_bpin_out 1)
  (bind _aspin_bpin_out_2 (Utilities|Casting|CastTopinBPInOut (Variables|/Script/Engine.ChildActorComponent|GetChildActor (Variables|Default|GetpinBPInOut0))))
  (Default|SetMain _aspin_bpin_out_2 self)
  (Variables|/Game/Final_Breadboard_Demo2/Actors/Other_Actors/pinBPInOut.pinBPInOut_C|SetpinID _aspin_bpin_out_2 0))