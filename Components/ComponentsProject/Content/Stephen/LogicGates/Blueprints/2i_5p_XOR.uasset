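; Two-input XOR logic gate Blueprint that passes a boolean signal on to the next connected Blueprint.
; GetPin1 and GetPin2 each store their input, then run a shared evaluation that is true when exactly one pin is high.
; The result is saved in PinValue and pushed to PinOut through GetValueOutput on every input event, so updates are event-driven.
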(event Custom|Get%20Pin%201
  (params (Pin1 :type Boolean))
  ;[1 1 1] Create input events / set pins
  (bind _output_get (Variables|Default|SetPin1 Pin1))
  ;[1 1 1] 2 Input 2 Circuit XOR Gate
  (if (or (and _output_get (not (stale Custom|Get%20Pin%202 _output_get))) (and (not _output_get) (stale Custom|Get%20Pin%202 _output_get)))
    ;[1 1 1] Send Output to next blueprint - Boolean
    (Variables|Default|SetPin%20Value true)
    (Default|GetValueOutput (Variables|Default|GetPin%20out) (Variables|Default|GetPin%20Value))
    (else
      (Variables|Default|SetPin%20Value false)
      (Default|GetValueOutput (Variables|Default|GetPin%20out) (Variables|Default|GetPin%20Value)))))

(event Custom|Get%20Pin%202
  (params (Pin2 :type Boolean))
  ;[1 1 1] Create input events / set pins
  (bind _output_get (Variables|Default|SetPin2 Pin2))
  ;[1 1 1] 2 Input 2 Circuit XOR Gate
  (if (or (and (stale Custom|Get%20Pin%201 _output_get) (not _output_get)) (and (not (stale Custom|Get%20Pin%201 _output_get)) _output_get))
    ;[1 1 1] Send Output to next blueprint - Boolean
    (Variables|Default|SetPin%20Value true)
    (Default|GetValueOutput (Variables|Default|GetPin%20out) (Variables|Default|GetPin%20Value))
    (else
      (Variables|Default|SetPin%20Value false)
      (Default|GetValueOutput (Variables|Default|GetPin%20out) (Variables|Default|GetPin%20Value)))))

(fn ConstructionScript)