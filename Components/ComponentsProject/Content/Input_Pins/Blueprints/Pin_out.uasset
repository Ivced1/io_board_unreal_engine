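; Pin_out is an output pin Blueprint that displays a Boolean value in the game.
; Its get_value_output event stores the incoming value in PinOut and colors the Pin mesh green for true or red for false.
; The same branch toggles two text renders as a 1 or 0 overlay matching that state.
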(event Custom|get_value_output
  (params (Pin_Value :type Boolean))
  (bind _pin (Variables|Default|GetPin))
  ;[1 1 1] Get Pin Output Value - Boolean
  (bind _output_get (Variables|Default|SetPin_Out Pin_Value))
  (if _output_get
    (Rendering|Material|SetMaterial _pin 0 "/Game/Input_Pins/Materials/Green.Green")
    ;[1 1 1] Just for fun. Used 1 or 0 overlay.
    (Rendering|SetVisibility (Variables|Default|GetTextRender0) false false)
    (Rendering|SetVisibility (Variables|Default|GetTextRender1) true false)
    (else
      (Rendering|Material|SetMaterial _pin 0 "/Game/Input_Pins/Materials/Red.Red")
      (Rendering|SetVisibility (Variables|Default|GetTextRender1) false false)
      (Rendering|SetVisibility (Variables|Default|GetTextRender0) true false))))

(fn ConstructionScript)