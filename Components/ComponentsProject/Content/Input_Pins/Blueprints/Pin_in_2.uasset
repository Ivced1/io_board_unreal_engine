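; Input pin actor that lets the player feed a Boolean into a 6i8pNAND logic gate.
; Overlapping the actor enables player input, and leaving disables it.
; Key 2 drives a FlipFlop that toggles PinIn and swaps the pin material between green and red.
; Only the true state is sent to the gate's PinOut via GetValueOutput; the false branch sends nothing.
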(event Collision|EventActorBeginOverlap
  (params (OtherActor :type Actor%20Object%20Reference))
  ;[1 1 1] Enable / Disable Player Controller
  (Input|EnableInput (Game|GetPlayerController 0)))

(event Collision|EventActorEndOverlap
  (params (OtherActor :type Actor%20Object%20Reference))
  ;[1 1 1] Enable / Disable Player Controller
  (Input|DisableInput (Game|GetPlayerController 0)))

(event Input|KeyboardEvents|2
  (params (Key :type Key%20Structure :default "None"))
  ;[1 1 1] Pass Boolean Value to Logic Gate
  (:Pressed
    (Utilities|FlowControl|FlipFlop
      (:A
        (Variables|Default|SetPin_In true)
        (Rendering|Material|SetMaterial (Variables|Default|GetPin) 0 "/Game/Input_Pins/Materials/Green.Green")
        ;[1 1 1] Send value to next blueprint - Boolean. Change this to send signal to correct pin number.
        (Default|GetValueOutput (Variables|/Game/Acacia6i_8p_NAND/Input_Pins/Blueprints/6i_8p_NAND.6i_8p_NAND_C|GetPin_Out (Variables|Default|Get6i_8p_NAND)) (Variables|Default|GetPin_In)))
      (:B
        (Variables|Default|SetPin_In false)
        (Rendering|Material|SetMaterial (Variables|Default|GetPin) 0 "/Game/Input_Pins/Materials/Red.Red")))))

(fn ConstructionScript)