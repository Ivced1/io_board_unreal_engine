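; Two-input XOR logic gate Blueprint that takes boolean signals and passes the result to the next Blueprint in a circuit.
; GetPin1 and GetPin2 each store their pin value, then both re-evaluate the same exclusive-or check.
; The result is saved to PinValue and sent to the linked PinOut through GetValueOutput, so gates can chain together.
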(event Custom|Get%20Pin%201
  (params (Pin1 :type Boolean))
  ;[1 1 1] Create input events / set pins
  (bind _output_get (Variables|Default|SetPin%201 Pin1))
  ;[1 1 1] 2 Input 2 Circuit XOR Gate
  (if (or (and _output_get (not (stale Custom|Get%20Pin%202 _output_get))) (and (not _output_get) (stale Custom|Get%20Pin%202 _output_get)))
    ;[1 1 1] Send Output to next blueprint - Boolean
    (Variables|Default|SetPin_Value true)
    (Default|GetValueOutput (Variables|Default|GetPin%20out) (Variables|Default|GetPin_Value))
    (else
      (Variables|Default|SetPin_Value false)
      (Default|GetValueOutput (Variables|Default|GetPin%20out) (Variables|Default|GetPin_Value)))))

(event Custom|Get%20Pin%202
  (params (Pin2 :type Boolean))
  ;[1 1 1] Create input events / set pins
  (bind _output_get (Variables|Default|SetPin%202 Pin2))
  ;[1 1 1] 2 Input 2 Circuit XOR Gate
  (if (or (and (stale Custom|Get%20Pin%201 _output_get) (not _output_get)) (and (not (stale Custom|Get%20Pin%201 _output_get)) _output_get))
    ;[1 1 1] Send Output to next blueprint - Boolean
    (Variables|Default|SetPin_Value true)
    (Default|GetValueOutput (Variables|Default|GetPin%20out) (Variables|Default|GetPin_Value))
    (else
      (Variables|Default|SetPin_Value false)
      (Default|GetValueOutput (Variables|Default|GetPin%20out) (Variables|Default|GetPin_Value)))))

(event EventBeginPlay)

(event Collision|EventActorBeginOverlap
  (params (OtherActor :type Actor%20Object%20Reference)))

(event EventTick
  (params (DeltaSeconds :type Float%20%28single-precision%29)))

(fn ConstructionScript)