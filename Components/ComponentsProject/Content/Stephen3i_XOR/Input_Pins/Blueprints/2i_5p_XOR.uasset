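; Two-input XOR logic gate Blueprint for a boolean circuit built from linked Blueprints.
; GetPin1 and GetPin2 events each store an incoming value in the matching pin variable.
; An XOR branch sets PinValue and passes it to the next Blueprint through GetValueOutput on PinOut.
; That evaluation branch has no event driving it, so the gate never sends output as wired.
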(event Custom|Get%20Pin%201
  (params (Pin1 :type Boolean))
  ;[1 1 1] Create input events / set pins
  (bind _output_get (Variables|Default|SetPin1 Pin1)))

(event Custom|Get%20Pin%202
  (params (Pin2 :type Boolean))
  ;[1 1 1] Create input events / set pins
  (bind _output_get (Variables|Default|SetPin2 Pin2)))

(fn ConstructionScript)