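; Input pin actor that lets the player toggle a boolean fed into an XOR logic gate.
; Overlapping the actor enables input for player controller 0, and ending the overlap disables it.
; Pressing the 2 key alternates PinIn through a FlipFlop, recolors the pin green for true or red for false, and passes the value to the 2i5pXOR gate via GetPin2.
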(event Collision|EventActorBeginOverlap
  (params (OtherActor :type Actor%20Object%20Reference))
  ;[1 1 1] Enable / Disable Player Controller
  (Input|EnableInput (Game|GetPlayerController 0)))

(event Collision|EventActorEndOverlap
  (params (OtherActor :type Actor%20Object%20Reference))
  ;[1 1 1] Enable / Disable Player Controller
  (Input|DisableInput (Game|GetPlayerController 0)))

(event Input|KeyboardEvents|2
  (params (Key :type Key%20Structure :default "None"))
  ;[1 1 1] Pass Boolean Value to Logic Gate
  (:Pressed
    (Utilities|FlowControl|FlipFlop
      (:A
        (Variables|Default|SetPin_In true)
        (Rendering|Material|SetMaterial (Variables|Default|GetPin) 0 "/Game/Input_Pins/Materials/Green.Green")
        (Default|GetPin2 (Variables|Default|Get2i_5p_XOR) (Variables|Default|GetPin_In)))
      (:B
        (Variables|Default|SetPin_In false)
        (Rendering|Material|SetMaterial (Variables|Default|GetPin) 0 "/Game/Input_Pins/Materials/Red.Red")
        (Default|GetPin2 (Variables|Default|Get2i_5p_XOR) (Variables|Default|GetPin_In))))))

(fn ConstructionScript)