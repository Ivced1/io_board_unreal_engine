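; WireBP is a wire actor that passes power between its two in/out pins in either direction.
; The construction script gives both child-actor pins a reference to the wire and an ID of 0 or 1.
; PowerUpdate stores the incoming power as that pin ID's input, then casts the opposite end's child actor to pinBP and calls OutputPower with the value.
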(event EventPowerUpdate
  (params (power :type Boolean%20%28by%20ref%29) (pinNumber :type Integer%20%28by%20ref%29))
  ;[1 1 1] Based on the pinID set the input from that pin to the power status of the pin
  (switch int pinNumber
    (:0
      (bind _output_get (Variables|Default|Setinput0 power))
      ;[1 1 1] Update the power value of the opposite end's pin
      (bind _aspin_bp (Utilities|Casting|CastTopinBP (Variables|/Script/Engine.ChildActorComponent|GetChildActor (Variables|Default|GetpinBPInOut1))))
      (Default|OutputPower _aspin_bp _output_get))
    (:1
      (bind _output_get_2 (Variables|Default|Setinput1 power))
      (bind _aspin_bp_2 (Utilities|Casting|CastTopinBP (Variables|/Script/Engine.ChildActorComponent|GetChildActor (Variables|Default|GetpinBPInOut0))))
      (Default|OutputPower _aspin_bp_2 _output_get_2))))

(fn ConstructionScript
  (|CallParentFunction)
  ;[1 1 1] Set Pin1's PinID and sets it's main component reference to the wire
  (bind _aspin_bpin_out (Utilities|Casting|CastTopinBPInOut (Variables|/Script/Engine.ChildActorComponent|GetChildActor (Variables|Default|GetpinBPInOut1))))
  (Default|SetMain _aspin_bpin_out self)
  (Variables|/Game/Peter/Full-InterobjectEventCalling/pinBPInOut.pinBPInOut_C|SetpinID _aspin_bpin_out 1)
  ;[1 1 1] Set Pin0's PinID and sets it's main component reference to the wire
  (bind _aspin_bpin_out_2 (Utilities|Casting|CastTopinBPInOut (Variables|/Script/Engine.ChildActorComponent|GetChildActor (Variables|Default|GetpinBPInOut0))))
  (Default|SetMain _aspin_bpin_out_2 self)
  (Variables|/Game/Peter/Full-InterobjectEventCalling/pinBPInOut.pinBPInOut_C|SetpinID _aspin_bpin_out_2 0))