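; Three-input AND logic gate Blueprint that acts as a circuit component, passing a boolean result to another object.
; Each input pin event stores its value, then re-evaluates the AND of all three pins.
; The result is pushed downstream on every input through GetValueOutput on the PinOut reference, so propagation is event-driven with no Tick logic.
; A SetOutputPin function offers a branch-based output path but is not called in this graph.
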(event Custom|Get_Pin_3
  (params (Pin3 :type Boolean))
  ;[1 1 1] Create input events / set pins (BASED ON CHILD)
  (bind _output_get (Variables|Default|SetPin%203 Pin3))
  (Default|GetValueOutput (Variables|Default|GetPin_Out) (and (and (stale Custom|Get_Pin_1 _output_get) (stale Custom|Get_Pin_2 _output_get)) _output_get)))

(event Custom|Get_Pin_1
  (params (Pin1 :type Boolean))
  ;[1 1 1] Create input events / set pins (BASED ON CHILD)
  (bind _output_get (Variables|Default|SetPin%201 Pin1))
  (Default|GetValueOutput (Variables|Default|GetPin_Out) (and (and _output_get (stale Custom|Get_Pin_2 _output_get)) (stale Custom|Get_Pin_3 _output_get))))

(event Custom|Get_Pin_2
  (params (Pin2 :type Boolean))
  ;[1 1 1] Create input events / set pins (BASED ON CHILD)
  (bind _output_get (Variables|Default|SetPin%202 Pin2))
  (Default|GetValueOutput (Variables|Default|GetPin_Out) (and (and (stale Custom|Get_Pin_1 _output_get) _output_get) (stale Custom|Get_Pin_3 _output_get))))

(event EventBeginPlay)

(event Collision|EventActorBeginOverlap
  (params (OtherActor :type Actor%20Object%20Reference)))

(event EventTick
  (params (DeltaSeconds :type Float%20%28single-precision%29)))

(fn ConstructionScript)

(fn SetOutputPin
  (params (Condition :type Boolean))
  ;[1 1 1] 3 Input 2 Circuit AND Gate - Boolean
  (if Condition
    ;[1 1 1] Send Output to next blueprint - Boolean
    (Variables|Default|SetPin_Value true)
    (else
      (Variables|Default|SetPin_Value false)))
  (Default|GetValueOutput (Variables|Default|GetPin_Out) (Variables|Default|GetPin_Value)))